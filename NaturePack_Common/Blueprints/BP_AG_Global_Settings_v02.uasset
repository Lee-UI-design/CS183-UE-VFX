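; Global settings actor for the nature pack that drives wind, tint noise, SSS, AO and top-layer looks for foliage and prop materials.
; It writes its variables into Global, Tree, Grass and Props Material Parameter Collections, taking wind direction from the AGGlobalSettings component's forward vector.
; The same writes run in Construction Script and BeginPlay.
; BeginPlay adds two Landscape TopLayer writes with no collection assigned.
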(event `self.ReceiveBeginPlay`
  ;[1 1 1] AG Arrow Direction
  (`KismetMaterialLibrary.SetVectorParameterValue` "/Game/ANGRY_MESH/NaturePack_Common/Materials/Collections/MPC_AG_Global_01.MPC_AG_Global_01" "Wind Arrow Direction" (`KismetMathLibrary.Conv_VectorToLinearColor` (`KismetMathLibrary.Conv_RotatorToVector` (`SceneComponent.RelativeRotation` (`self.AG_Global_Settings`)))))
  ;[1 1 1] AG Global Wind Parameters
  (`KismetMaterialLibrary.SetScalarParameterValue` "/Game/ANGRY_MESH/NaturePack_Common/Materials/Collections/MPC_AG_MTree_01.MPC_AG_MTree_01" "Wind Tree Amplitude" (`self.Wind Tree Amplitude`))
  (`KismetMaterialLibrary.SetScalarParameterValue` "/Game/ANGRY_MESH/NaturePack_Common/Materials/Collections/MPC_AG_MTree_01.MPC_AG_MTree_01" "Wind Tree Speed" (`self.Wind Tree Speed`))
  (`KismetMaterialLibrary.SetScalarParameterValue` "/Game/ANGRY_MESH/NaturePack_Common/Materials/Collections/MPC_AG_MTree_01.MPC_AG_MTree_01" "Wind Tree Flexibility" (`self.Wind Tree Flexibility`))
  (`KismetMaterialLibrary.SetScalarParameterValue` "/Game/ANGRY_MESH/NaturePack_Common/Materials/Collections/MPC_AG_MTree_01.MPC_AG_MTree_01" "Wind Tree Leaf Amplitude" (`self.Wind Tree Leaf Amplitude`))
  (`KismetMaterialLibrary.SetScalarParameterValue` "/Game/ANGRY_MESH/NaturePack_Common/Materials/Collections/MPC_AG_MTree_01.MPC_AG_MTree_01" "Wind Tree Leaf Speed" (`self.Wind Tree Leaf Speed`))
  (`KismetMaterialLibrary.SetScalarParameterValue` "/Game/ANGRY_MESH/NaturePack_Common/Materials/Collections/MPC_AG_MTree_01.MPC_AG_MTree_01" "Wind Tree Leaf Turbulence" (`self.Wind Tree Leaf Turbulence`))
  (`KismetMaterialLibrary.SetScalarParameterValue` "/Game/ANGRY_MESH/NaturePack_Common/Materials/Collections/MPC_AG_MTree_01.MPC_AG_MTree_01" "Wind Tree Leaf Flexibility" (`self.Wind Tree Leaf Flexibility`))
  (`KismetMaterialLibrary.SetScalarParameterValue` "/Game/ANGRY_MESH/NaturePack_Common/Materials/Collections/MPC_AG_MGrass_01.MPC_AG_MGrass_01" "Wind Grass Amplitude" (`self.Wind Grass Amplitude`))
  (`KismetMaterialLibrary.SetScalarParameterValue` "/Game/ANGRY_MESH/NaturePack_Common/Materials/Collections/MPC_AG_MGrass_01.MPC_AG_MGrass_01" "Wind Grass Speed" (`self.Wind Grass Speed`))
  (`KismetMaterialLibrary.SetScalarParameterValue` "/Game/ANGRY_MESH/NaturePack_Common/Materials/Collections/MPC_AG_MGrass_01.MPC_AG_MGrass_01" "Wind Grass Turbulence" (`self.Wind Grass Turbulence`))
  (`KismetMaterialLibrary.SetScalarParameterValue` "/Game/ANGRY_MESH/NaturePack_Common/Materials/Collections/MPC_AG_MGrass_01.MPC_AG_MGrass_01" "Wind Grass Flexibility" (`self.Wind Grass Flexibility`))
  (`KismetMaterialLibrary.SetScalarParameterValue` "/Game/ANGRY_MESH/NaturePack_Common/Materials/Collections/MPC_AG_MGrass_01.MPC_AG_MGrass_01" "Wind Grass Waves Amplitude" (`self.Wind Grass Waves Amplitude`))
  (`KismetMaterialLibrary.SetScalarParameterValue` "/Game/ANGRY_MESH/NaturePack_Common/Materials/Collections/MPC_AG_MGrass_01.MPC_AG_MGrass_01" "Wind Grass Waves Speed" (`self.Wind Grass Waves Speed`))
  (`KismetMaterialLibrary.SetScalarParameterValue` "/Game/ANGRY_MESH/NaturePack_Common/Materials/Collections/MPC_AG_MGrass_01.MPC_AG_MGrass_01" "Wind Grass Waves Scale" (`self.Wind Grass Waves Scale`))
  ;[1 1 1] AG Global Parameters
  (`KismetMaterialLibrary.SetScalarParameterValue` "/Game/ANGRY_MESH/NaturePack_Common/Materials/Collections/MPC_AG_Global_01.MPC_AG_Global_01" "Global Top Layer Height Start" (`self.Global Top Layer Height Start`))
  (`KismetMaterialLibrary.SetScalarParameterValue` "/Game/ANGRY_MESH/NaturePack_Common/Materials/Collections/MPC_AG_Global_01.MPC_AG_Global_01" "Global Top Layer Height Fade" (`self.Global Top Layer Height Fade`))
  (`KismetMaterialLibrary.SetScalarParameterValue` "/Game/ANGRY_MESH/NaturePack_Common/Materials/Collections/MPC_AG_Global_01.MPC_AG_Global_01" "Global Tint Noise UV Scale" (`self.Global Tint Noise UV Scale`))
  (`KismetMaterialLibrary.SetScalarParameterValue` "/Game/ANGRY_MESH/NaturePack_Common/Materials/Collections/MPC_AG_Global_01.MPC_AG_Global_01" "Global Tint Noise Intensity" (`self.Global Tint Noise Intensity`))
  (`KismetMaterialLibrary.SetScalarParameterValue` "/Game/ANGRY_MESH/NaturePack_Common/Materials/Collections/MPC_AG_Global_01.MPC_AG_Global_01" "Global Tint Noise Contrast" (`self.Global Tint Noise Contrast`))
  (`KismetMaterialLibrary.SetScalarParameterValue` "/Game/ANGRY_MESH/NaturePack_Common/Materials/Collections/MPC_AG_MTree_01.MPC_AG_MTree_01" "Global Tree SSS Intensity" (`self.Global Tree SSS Intensity`))
  (`KismetMaterialLibrary.SetScalarParameterValue` "/Game/ANGRY_MESH/NaturePack_Common/Materials/Collections/MPC_AG_MTree_01.MPC_AG_MTree_01" "Global Tree SSS AO Influence" (`self.Global Tree SSS AO Influence`))
  (`KismetMaterialLibrary.SetScalarParameterValue` "/Game/ANGRY_MESH/NaturePack_Common/Materials/Collections/MPC_AG_MTree_01.MPC_AG_MTree_01" "Global Tree AO" (`self.Global Tree AO`))
  (`KismetMaterialLibrary.SetScalarParameterValue` "/Game/ANGRY_MESH/NaturePack_Common/Materials/Collections/MPC_AG_MGrass_01.MPC_AG_MGrass_01" "Global Grass SSS Intensity" (`self.Global Grass SSS Intensity`))
  (`KismetMaterialLibrary.SetScalarParameterValue` "/Game/ANGRY_MESH/NaturePack_Common/Materials/Collections/MPC_AG_MGrass_01.MPC_AG_MGrass_01" "Global Grass SSS AO Influence" (`self.Global Grass SSS AO Influence`))
  ;[1 1 1] AG Global Top Layer Parameters
  (`KismetMaterialLibrary.SetScalarParameterValue` "/Game/ANGRY_MESH/NaturePack_Common/Materials/Collections/MPC_AG_MTree_01.MPC_AG_MTree_01" "Top Layer Tree Intensity" (`self.Top Layer Tree Intensity`))
  (`KismetMaterialLibrary.SetScalarParameterValue` "/Game/ANGRY_MESH/NaturePack_Common/Materials/Collections/MPC_AG_MTree_01.MPC_AG_MTree_01" "Top Layer Tree Offset" (`self.Top Layer Tree Offset`))
  (`KismetMaterialLibrary.SetScalarParameterValue` "/Game/ANGRY_MESH/NaturePack_Common/Materials/Collections/MPC_AG_MTree_01.MPC_AG_MTree_01" "Top Layer Tree Contast" (`self.Top Layer Tree Contast`))
  (`KismetMaterialLibrary.SetScalarParameterValue` "/Game/ANGRY_MESH/NaturePack_Common/Materials/Collections/MPC_AG_MTree_01.MPC_AG_MTree_01" "Top Layer Tree Arrow Offset" (`self.Top Layer Tree Arrow Offset`))
  (`KismetMaterialLibrary.SetScalarParameterValue` "/Game/ANGRY_MESH/NaturePack_Common/Materials/Collections/MPC_AG_MProps_01.MPC_AG_MProps_01" "Top Layer Props Intensity" (`self.Top Layer Props Intensity`))
  (`KismetMaterialLibrary.SetScalarParameterValue` "/Game/ANGRY_MESH/NaturePack_Common/Materials/Collections/MPC_AG_MProps_01.MPC_AG_MProps_01" "Top Layer Props Offset" (`self.Top Layer Props Offset`))
  (`KismetMaterialLibrary.SetScalarParameterValue` "/Game/ANGRY_MESH/NaturePack_Common/Materials/Collections/MPC_AG_MProps_01.MPC_AG_MProps_01" "Top Layer Props Contrast" (`self.Top Layer Props Contrast`))
  (`KismetMaterialLibrary.SetScalarParameterValue` "/Game/ANGRY_MESH/NaturePack_Common/Materials/Collections/MPC_AG_MGrass_01.MPC_AG_MGrass_01" "Top Layer Grass Intensity" (`self.Top Layer Grass Intensity`))
  (`KismetMaterialLibrary.SetScalarParameterValue` "/Game/ANGRY_MESH/NaturePack_Common/Materials/Collections/MPC_AG_MGrass_01.MPC_AG_MGrass_01" "Top Layer Grass Offset" (`self.Top Layer Grass Offset`))
  (`KismetMaterialLibrary.SetScalarParameterValue` "/Game/ANGRY_MESH/NaturePack_Common/Materials/Collections/MPC_AG_MGrass_01.MPC_AG_MGrass_01" "Top Layer Grass Contast" (`self.Top Layer Grass Contrast`))
  (`KismetMaterialLibrary.SetScalarParameterValue` null "Landscape TopLayer Offset")
  (`KismetMaterialLibrary.SetScalarParameterValue` null "Landscape TopLayer Contrast"))

(fn `UserConstructionScript`
  ;[1 1 1] AG Arrow Direction
  (`KismetMaterialLibrary.SetVectorParameterValue` "/Game/ANGRY_MESH/NaturePack_Common/Materials/Collections/MPC_AG_Global_01.MPC_AG_Global_01" "Wind Arrow Direction" (`KismetMathLibrary.Conv_VectorToLinearColor` (`KismetMathLibrary.Conv_RotatorToVector` (`SceneComponent.RelativeRotation` (`self.AG_Global_Settings`)))))
  ;[1 1 1] AG Global Wind Parameters
  (`KismetMaterialLibrary.SetScalarParameterValue` "/Game/ANGRY_MESH/NaturePack_Common/Materials/Collections/MPC_AG_MTree_01.MPC_AG_MTree_01" "Wind Tree Amplitude" (`self.Wind Tree Amplitude`))
  (`KismetMaterialLibrary.SetScalarParameterValue` "/Game/ANGRY_MESH/NaturePack_Common/Materials/Collections/MPC_AG_MTree_01.MPC_AG_MTree_01" "Wind Tree Speed" (`self.Wind Tree Speed`))
  (`KismetMaterialLibrary.SetScalarParameterValue` "/Game/ANGRY_MESH/NaturePack_Common/Materials/Collections/MPC_AG_MTree_01.MPC_AG_MTree_01" "Wind Tree Flexibility" (`self.Wind Tree Flexibility`))
  (`KismetMaterialLibrary.SetScalarParameterValue` "/Game/ANGRY_MESH/NaturePack_Common/Materials/Collections/MPC_AG_MTree_01.MPC_AG_MTree_01" "Wind Tree Leaf Amplitude" (`self.Wind Tree Leaf Amplitude`))
  (`KismetMaterialLibrary.SetScalarParameterValue` "/Game/ANGRY_MESH/NaturePack_Common/Materials/Collections/MPC_AG_MTree_01.MPC_AG_MTree_01" "Wind Tree Leaf Speed" (`self.Wind Tree Leaf Speed`))
  (`KismetMaterialLibrary.SetScalarParameterValue` "/Game/ANGRY_MESH/NaturePack_Common/Materials/Collections/MPC_AG_MTree_01.MPC_AG_MTree_01" "Wind Tree Leaf Turbulence" (`self.Wind Tree Leaf Turbulence`))
  (`KismetMaterialLibrary.SetScalarParameterValue` "/Game/ANGRY_MESH/NaturePack_Common/Materials/Collections/MPC_AG_MTree_01.MPC_AG_MTree_01" "Wind Tree Leaf Flexibility" (`self.Wind Tree Leaf Flexibility`))
  (`KismetMaterialLibrary.SetScalarParameterValue` "/Game/ANGRY_MESH/NaturePack_Common/Materials/Collections/MPC_AG_MGrass_01.MPC_AG_MGrass_01" "Wind Grass Amplitude" (`self.Wind Grass Amplitude`))
  (`KismetMaterialLibrary.SetScalarParameterValue` "/Game/ANGRY_MESH/NaturePack_Common/Materials/Collections/MPC_AG_MGrass_01.MPC_AG_MGrass_01" "Wind Grass Speed" (`self.Wind Grass Speed`))
  (`KismetMaterialLibrary.SetScalarParameterValue` "/Game/ANGRY_MESH/NaturePack_Common/Materials/Collections/MPC_AG_MGrass_01.MPC_AG_MGrass_01" "Wind Grass Turbulence" (`self.Wind Grass Turbulence`))
  (`KismetMaterialLibrary.SetScalarParameterValue` "/Game/ANGRY_MESH/NaturePack_Common/Materials/Collections/MPC_AG_MGrass_01.MPC_AG_MGrass_01" "Wind Grass Flexibility" (`self.Wind Grass Flexibility`))
  (`KismetMaterialLibrary.SetScalarParameterValue` "/Game/ANGRY_MESH/NaturePack_Common/Materials/Collections/MPC_AG_MGrass_01.MPC_AG_MGrass_01" "Wind Grass Waves Amplitude" (`self.Wind Grass Waves Amplitude`))
  (`KismetMaterialLibrary.SetScalarParameterValue` "/Game/ANGRY_MESH/NaturePack_Common/Materials/Collections/MPC_AG_MGrass_01.MPC_AG_MGrass_01" "Wind Grass Waves Speed" (`self.Wind Grass Waves Speed`))
  (`KismetMaterialLibrary.SetScalarParameterValue` "/Game/ANGRY_MESH/NaturePack_Common/Materials/Collections/MPC_AG_MGrass_01.MPC_AG_MGrass_01" "Wind Grass Waves Scale" (`self.Wind Grass Waves Scale`))
  ;[1 1 1] AG Global Parameters
  (`KismetMaterialLibrary.SetScalarParameterValue` "/Game/ANGRY_MESH/NaturePack_Common/Materials/Collections/MPC_AG_Global_01.MPC_AG_Global_01" "Global Top Layer Height Start" (`self.Global Top Layer Height Start`))
  (`KismetMaterialLibrary.SetScalarParameterValue` "/Game/ANGRY_MESH/NaturePack_Common/Materials/Collections/MPC_AG_Global_01.MPC_AG_Global_01" "Global Top Layer Height Fade" (`self.Global Top Layer Height Fade`))
  (`KismetMaterialLibrary.SetScalarParameterValue` "/Game/ANGRY_MESH/NaturePack_Common/Materials/Collections/MPC_AG_Global_01.MPC_AG_Global_01" "Global Tint Noise UV Scale" (`self.Global Tint Noise UV Scale`))
  (`KismetMaterialLibrary.SetScalarParameterValue` "/Game/ANGRY_MESH/NaturePack_Common/Materials/Collections/MPC_AG_Global_01.MPC_AG_Global_01" "Global Tint Noise Intensity" (`self.Global Tint Noise Intensity`))
  (`KismetMaterialLibrary.SetScalarParameterValue` "/Game/ANGRY_MESH/NaturePack_Common/Materials/Collections/MPC_AG_Global_01.MPC_AG_Global_01" "Global Tint Noise Contrast" (`self.Global Tint Noise Contrast`))
  (`KismetMaterialLibrary.SetScalarParameterValue` "/Game/ANGRY_MESH/NaturePack_Common/Materials/Collections/MPC_AG_MTree_01.MPC_AG_MTree_01" "Global Tree SSS Intensity" (`self.Global Tree SSS Intensity`))
  (`KismetMaterialLibrary.SetScalarParameterValue` "/Game/ANGRY_MESH/NaturePack_Common/Materials/Collections/MPC_AG_MTree_01.MPC_AG_MTree_01" "Global Tree SSS AO Influence" (`self.Global Tree SSS AO Influence`))
  (`KismetMaterialLibrary.SetScalarParameterValue` "/Game/ANGRY_MESH/NaturePack_Common/Materials/Collections/MPC_AG_MTree_01.MPC_AG_MTree_01" "Global Tree AO" (`self.Global Tree AO`))
  (`KismetMaterialLibrary.SetScalarParameterValue` "/Game/ANGRY_MESH/NaturePack_Common/Materials/Collections/MPC_AG_MGrass_01.MPC_AG_MGrass_01" "Global Grass SSS Intensity" (`self.Global Grass SSS Intensity`))
  (`KismetMaterialLibrary.SetScalarParameterValue` "/Game/ANGRY_MESH/NaturePack_Common/Materials/Collections/MPC_AG_MGrass_01.MPC_AG_MGrass_01" "Global Grass SSS AO Influence" (`self.Global Grass SSS AO Influence`))
  ;[1 1 1] AG Global Top Layer Parameters
  (`KismetMaterialLibrary.SetScalarParameterValue` "/Game/ANGRY_MESH/NaturePack_Common/Materials/Collections/MPC_AG_MTree_01.MPC_AG_MTree_01" "Top Layer Tree Intensity" (`self.Top Layer Tree Intensity`))
  (`KismetMaterialLibrary.SetScalarParameterValue` "/Game/ANGRY_MESH/NaturePack_Common/Materials/Collections/MPC_AG_MTree_01.MPC_AG_MTree_01" "Top Layer Tree Offset" (`self.Top Layer Tree Offset`))
  (`KismetMaterialLibrary.SetScalarParameterValue` "/Game/ANGRY_MESH/NaturePack_Common/Materials/Collections/MPC_AG_MTree_01.MPC_AG_MTree_01" "Top Layer Tree Contast" (`self.Top Layer Tree Contast`))
  (`KismetMaterialLibrary.SetScalarParameterValue` "/Game/ANGRY_MESH/NaturePack_Common/Materials/Collections/MPC_AG_MTree_01.MPC_AG_MTree_01" "Top Layer Tree Arrow Offset" (`self.Top Layer Tree Arrow Offset`))
  (`KismetMaterialLibrary.SetScalarParameterValue` "/Game/ANGRY_MESH/NaturePack_Common/Materials/Collections/MPC_AG_MProps_01.MPC_AG_MProps_01" "Top Layer Props Intensity" (`self.Top Layer Props Intensity`))
  (`KismetMaterialLibrary.SetScalarParameterValue` "/Game/ANGRY_MESH/NaturePack_Common/Materials/Collections/MPC_AG_MProps_01.MPC_AG_MProps_01" "Top Layer Props Offset" (`self.Top Layer Props Offset`))
  (`KismetMaterialLibrary.SetScalarParameterValue` "/Game/ANGRY_MESH/NaturePack_Common/Materials/Collections/MPC_AG_MProps_01.MPC_AG_MProps_01" "Top Layer Props Contrast" (`self.Top Layer Props Contrast`))
  (`KismetMaterialLibrary.SetScalarParameterValue` "/Game/ANGRY_MESH/NaturePack_Common/Materials/Collections/MPC_AG_MGrass_01.MPC_AG_MGrass_01" "Top Layer Grass Intensity" (`self.Top Layer Grass Intensity`))
  (`KismetMaterialLibrary.SetScalarParameterValue` "/Game/ANGRY_MESH/NaturePack_Common/Materials/Collections/MPC_AG_MGrass_01.MPC_AG_MGrass_01" "Top Layer Grass Offset" (`self.Top Layer Grass Offset`))
  (`KismetMaterialLibrary.SetScalarParameterValue` "/Game/ANGRY_MESH/NaturePack_Common/Materials/Collections/MPC_AG_MGrass_01.MPC_AG_MGrass_01" "Top Layer Grass Contast" (`self.Top Layer Grass Contrast`)))